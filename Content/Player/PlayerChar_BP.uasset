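; Player character Blueprint for a shooter against AI characters, with movement, mouse look, jumping, health and score.
; Holding Fire runs a looping timer that spawns projectiles from an arrow component.
; Damage updates the HUD widget; death by an AI character awards it a point through a DoOnce gate and respawns the player at a random SpawnPoint, resetting the gate.
; Holding ShowScore displays a score widget.
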(event Custom|CheckHP
  ;[0 0 0] Health and Damage
  (if (<= (Variables|Default|GetHealth) 0.0)
    (bind _asaichar_bp (Utilities|Casting|CastToAIChar_BP (Variables|Default|GetDamage%20Causer)))
    (Utilities|FlowControl|DoOnce false
      (:Completed
        (Default|AddScore _asaichar_bp 1)
        (CallFunction|Respawn)))))

(event Custom|Respawn
  (bind _spawnpoints (Variables|Default|GetSpawnPoints))
  ;[0 0 0] Respawn
  (Variables|Default|SetHealth 1e+02)
  (Transformation|SetActorLocation (Transformation|GetActorLocation (Utilities|Array|Get(acopy) _spawnpoints (Math|Random|RandomIntegerinRange 0 (- (Utilities|Array|Length _spawnpoints) 1)))) false true)
  (CallFunction|ResetDoOnce))

(event Custom|AddScore
  (params (Value :type Integer))
  ;[0 0 0] AddScore
  (Variables|Default|SetScore (+ (Variables|Default|GetScore) Value)))

(event Custom|ResetDoOnce
  ;[0 0 0] Health and Damage
  (Utilities|FlowControl|DoOnce false) ; enters at Reset
)

(event Custom|HealthBonus
  (params (MaxHealth :type Float%20%28double-precision%29))
  ;[0 0 0] Health and Damage
  (bind _output_get (Variables|Default|SetMaxHealth MaxHealth))
  (Variables|Default|SetHealth _output_get))

(event Custom|FireEvent
  ;[0 0 0] Fire Event
  (Game|SpawnActorfromClass "/Game/Player/PlayerProj_BP.PlayerProj_BP_C" (Transformation|GetWorldTransform (Variables|Default|GetArrow1)) "Undefined" "MultiplyWithRoot" self 0))

(event EventBeginPlay
  ;[0 0 0] Begin Play
  (bind _returnvalue (UserInterface|CreateWidget "/Game/Player/Player_W.Player_W_C"))
  (Variables|Default|SetPlayerWidget _returnvalue)
  (UserInterface|Viewport|AddtoViewport _returnvalue 0)
  (bind _outactors (Actor|GetAllActorsOfClass "/Game/Spawner/SpawnPoint.SpawnPoint_C"))
  (Variables|Default|SetSpawnPoints _outactors))

(event Game|Damage|EventAnyDamage
  (params (Damage :type Float%20%28single-precision%29) (DamageType :type Damage%20Type%20Object%20Reference) (InstigatedBy :type Controller%20Object%20Reference) (DamageCauser :type Actor%20Object%20Reference))
  ;[0 0 0] Health and Damage
  (Variables|Default|SetDamage%20Causer DamageCauser)
  (Variables|Default|SetHealth (- (Variables|Default|GetHealth) Damage))
  (CallFunction|CheckHP)
  (Default|SetHealth (Variables|Default|GetPlayerWidget) (Variables|Default|GetHealth) (Variables|Default|GetMaxHealth)))

(event Input|ActionEvents|InputActionJump
  (params (Key :type Key%20Structure :default "None"))
  ;[0 0 0] Jump Event
  (:Pressed
    (Character|Jump))
  (:Released
    (Character|StopJumping)))

(event Input|ActionEvents|InputActionFire
  (params (Key :type Key%20Structure :default "None"))
  ;[0 0 0] Fire Event
  (:Pressed
    (Utilities|Time|SetTimerbyFunctionName 0 "FireEvent" 0.1 true))
  (:Released
    (Utilities|Time|ClearTimerbyFunctionName 0 "FireEvent")))

(event Input|ActionEvents|InputActionShowScore
  (params (Key :type Key%20Structure :default "None"))
  ;[0 0 0] Show Score
  (:Pressed
    (bind _returnvalue (UserInterface|CreateWidget "/Game/Game/Score_W.Score_W_C" 0 self))
    (UserInterface|Viewport|AddtoViewport _returnvalue 0))
  (:Released
    (Widget|RemovefromParent _returnvalue)))

(event Input|AxisEvents|InputAxisMoveForward
  (params (AxisValue :type Float%20%28single-precision%29))
  ;[0 0 0] Movement
  (Pawn|Input|AddMovementInput (Math|Vector|GetForwardVector (Math|Rotator|MakeRotator 0.0 0.0 (.yaw (Pawn|GetControlRotation :!class /Script/Engine.Pawn)))) AxisValue false))

(event Input|AxisEvents|InputAxisMoveRight
  (params (AxisValue :type Float%20%28single-precision%29))
  (bind _returnvalue (Pawn|GetControlRotation :!class /Script/Engine.Pawn))
  ;[0 0 0] Movement
  (Pawn|Input|AddMovementInput (Math|Vector|GetRightVector (Math|Rotator|MakeRotator (.roll _returnvalue) 0.0 (.yaw _returnvalue))) AxisValue false))

(event Input|AxisEvents|InputAxisLookUp
  (params (AxisValue :type Float%20%28single-precision%29))
  ;[0 0 0] Mouse Look
  (Pawn|Input|AddControllerPitchInput AxisValue))

(event Input|AxisEvents|InputAxisTurn
  (params (AxisValue :type Float%20%28single-precision%29))
  ;[0 0 0] Mouse Look
  (Pawn|Input|AddControllerYawInput AxisValue))

(fn ConstructionScript)

(fn CheckHealth)