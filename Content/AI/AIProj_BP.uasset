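; AI projectile Blueprint that damages AI or player characters it overlaps, then destroys itself.
; The ProjectileOverlap component detects hits, counting AI characters only on their capsule and players on any component.
; Each branch uses a DoOnce to apply fixed damage once, with the projectile's owner as damage causer.
; Other overlaps are ignored, and a BeginPlay delay destroys the projectile after a few seconds.
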(event OnComponentBeginOverlap(ProjectileOverlap)
  (params (OverlappedComponent :type Primitive%20Component%20Object%20Reference) (OtherActor :type Actor%20Object%20Reference) (OtherComp :type Primitive%20Component%20Object%20Reference) (OtherBodyIndex :type Integer) (bFromSweep :type Boolean) (SweepResult :type Hit%20Result%20Structure%20%28by%20ref%29))
  (bind _returnvalue (Components|GetOwner))
  (bind _asaichar_bp (Utilities|Casting|CastToAICHAR_BP OtherActor)
    (:then
      (if (== (Variables|/Script/Engine.Character|GetCapsuleComponent _asaichar_bp) OtherComp)
        (Utilities|FlowControl|DoOnce false
          (:Completed
            (Game|Damage|ApplyDamage _asaichar_bp 1e+01 0 _returnvalue)
            (Actor|DestroyActor :!label _label)))))
    (:CastFailed
      (bind _asplayer_char_bp (Utilities|Casting|CastToPlayerChar_BP OtherActor))
      (Utilities|FlowControl|DoOnce false
        (:Completed
          (Game|Damage|ApplyDamage _asplayer_char_bp 1e+01 0 _returnvalue)
          (goto _label))))))

(event EventBeginPlay
  ;[0 0 0] Projectile Destructor
  (Utilities|FlowControl|Delay 3.0)
  (Actor|DestroyActor))

(fn ConstructionScript)